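; BP_Task_05_Character is a character that moves along a spline, previews its projectile's path and fires when the IA_Task5 input completes.
; While that input triggers, it predicts the path from the weapon muzzle with debug drawing, then aligns a spawned BP_HitPlace marker to the impact normal.
; MoveAlongSplineComponent handles movement, with speed-up and speed-down inputs adjusting it, and WeaponComponent supplies muzzle, velocity and firing.
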(event Input|EnhancedActionEvents|EnhancedInputActionIA_SpeedUp
  (params (ActionValue :type Boolean) (ElapsedSeconds :type Float%20%28double-precision%29) (TriggeredSeconds :type Float%20%28double-precision%29) (InputAction :type Input%20Action%20Object%20Reference :default "/Game/Basic/Input/Task5/IA_SpeedUp.IA_SpeedUp"))
  (:Started
    (Class|MoveAlongSplineComponent|AdjustSpeed (Variables|Default|GetMoveAlongSplineComponent) (Variables|Default|GetDeltaSpeed))))

(event Input|EnhancedActionEvents|EnhancedInputActionIA_SpeedDown
  (params (ActionValue :type Boolean) (ElapsedSeconds :type Float%20%28double-precision%29) (TriggeredSeconds :type Float%20%28double-precision%29) (InputAction :type Input%20Action%20Object%20Reference :default "/Game/Basic/Input/Task5/IA_SpeedDown.IA_SpeedDown"))
  (:Started
    (Class|MoveAlongSplineComponent|AdjustSpeed (Variables|Default|GetMoveAlongSplineComponent) (* (Variables|Default|GetDeltaSpeed) -1.0))))

(event Input|EnhancedActionEvents|EnhancedInputActionIA_Task5
  (params (ActionValue :type Boolean) (ElapsedSeconds :type Float%20%28double-precision%29) (TriggeredSeconds :type Float%20%28double-precision%29) (InputAction :type Input%20Action%20Object%20Reference :default "/Game/Basic/Input/Task5/IA_Task5.IA_Task5"))
  (:Triggered
    (CallFunction|UpdateTrajectory)
    (CallFunction|UpdateHitPlace))
  (:Completed
    (Class|WeaponComponent|Fire (Variables|Default|GetWeaponComponent))))

(event EventBeginPlay
  (bind _returnvalue (Game|SpawnActorfromClass "/Game/Task_05/BP_HitPlace.BP_HitPlace_C" (Math|Transform|MakeTransform "0.000000,0.000000,-100.000000" "0, 0, 0" "1.000000,1.000000,1.000000") "Undefined" "MultiplyWithRoot" 0 0))
  (Variables|Default|SetHitPlace _returnvalue)
  (Class|MoveAlongSplineComponent|Start (Variables|Default|GetMoveAlongSplineComponent)))

(fn ConstructionScript)

(fn UpdateTrajectory
  (bind (_predictresult _returnvalue) (Class|GameplayStatics|BlueprintPredictProjectilePathAdvanced (Utilities|Struct|MakePredictProjectilePathParams (.OutMuzzleLocation (Class|WeaponComponent|GetMuzzleTransform (Variables|Default|GetWeaponComponent))) (Class|WeaponComponent|GetProjectileVelocity (Variables|Default|GetWeaponComponent)) true 1e+01 3.0 true "ECC_WorldStatic" "ObjectTypeQuery1" 0 15.0 0.0 "ForDuration" 0.0 false)))
  (Variables|Default|SetbPredictSuccessful _returnvalue)
  (Variables|Default|SetPredictResut _predictresult))

(fn UpdateHitPlace
  (bind _predictresut (Variables|Default|GetPredictResut))
  (if (Variables|Default|GetbPredictSuccessful)
    (Transformation|SetActorTransform (Variables|Default|GetHitPlace) (Math|Transform|MakeTransform (.impactpoint (.hitresult _predictresut)) (Math|Rotator|MakeRotfromZ (.normal (.hitresult _predictresut)))) false true)))