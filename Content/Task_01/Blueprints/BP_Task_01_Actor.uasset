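; BP_Task_01_Actor is an interactable actor whose sphere turns orange the first time it is interacted with.
; Interact runs once, creating a dynamic material instance on the sphere and setting its Color parameter.
; PreInteract creates the label widget on first call and shows its widget component on later calls, while PostInteract hides it.
; GetObservationLocation returns the actor's location.
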(event EventBeginPlay)

(event Collision|EventActorBeginOverlap
  (params (OtherActor :type Actor%20Object%20Reference)))

(event EventTick
  (params (DeltaSeconds :type Float%20%28single-precision%29)))

(event EventInteract
  (bind _sphere (Variables|Default|GetSphere))
  (Utilities|FlowControl|DoOnce false
    (:Completed
      (bind _returnvalue (Rendering|Material|CreateDynamicMaterialInstance _sphere 0 (Rendering|Material|GetMaterial _sphere 0) "None" :!class /Script/Engine.PrimitiveComponent))
      (Rendering|Material|SetVectorParameterValue _returnvalue "Color" "(R=1.000000,G=0.257856,B=0.000000,A=1.000000)" :!class /Script/Engine.MaterialInstanceDynamic))))

(event EventPreInteract
  (Utilities|IsValid (UserInterface|GetWidget (Variables|Default|GetInteractWidgetComponent))
    (:Is%20Valid
      (Rendering|SetVisibility (Variables|Default|GetInteractWidgetComponent) true false))
    (:Is%20Not%20Valid
      (bind _returnvalue (UserInterface|CreateWidget "/Game/Task_01/Widgets/W_Interact_Lable.W_Interact_Lable_C"))
      (UserInterface|SetWidget (Variables|Default|GetInteractWidgetComponent) _returnvalue))))

(event EventPostInteract
  (Rendering|SetVisibility (Variables|Default|GetInteractWidgetComponent) false false))

(fn ConstructionScript)

(fn GetObservationLocation
  (return (Transformation|GetActorLocation)))